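; BP_Piece is a pickup-style piece actor that, when the player pawn overlaps it, calls ChangeScale(false) on BP_MyPawn and destroys itself.
; Collision stays off for the first 0.2 seconds after spawn, then switches to query-only so overlaps can register.
; On destruction it removes itself from the Pieces list of its Plane reference, if that is valid.
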(event `self.ReceiveBeginPlay`
  (bind _staticmesh (`self.StaticMesh`))
  (`PrimitiveComponent.SetCollisionEnabled` _staticmesh "NoCollision")
  (`KismetSystemLibrary.Delay` 0.2)
  (`PrimitiveComponent.SetCollisionEnabled` _staticmesh "QueryOnly"))

(event `self.StaticMesh.OnComponentBeginOverlap`
  (params (OverlappedComponent :type "PrimitiveComponent Object Reference") (OtherActor :type "Actor Object Reference") (OtherComp :type "PrimitiveComponent Object Reference") (OtherBodyIndex :type Integer) (bFromSweep :type Boolean) (SweepResult :type "HitResult Structure (by ref)"))
  (bind _asbp_my_pawn (cast `/Game/Blueprints/BP_MyPawn` OtherActor))
  (`/Game/Blueprints/BP_MyPawn.ChangeScale` _asbp_my_pawn false)
  (`self.K2_DestroyActor`))

(event `self.ReceiveDestroyed`
  (bind _plane (`self.Plane`))
  (if (`KismetSystemLibrary.IsValid` _plane)
    (`KismetArrayLibrary.Array_RemoveItem` (`/Game/Blueprints/BP_Plane.Pieces` _plane) self)))

(fn `UserConstructionScript`)