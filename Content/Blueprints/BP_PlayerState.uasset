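; BP_PlayerState is a player state that keeps a survival score which grows while the player is alive.
; A looping half-second timer started on BeginPlay runs Add Score, which increments MyScore if the controller's Alive flag is set.
; It finds that controller with GetActorOfClass, so it checks the first BP_MyPlayerController found rather than explicitly its owner.
; MyScore's RepNotify broadcasts OnScoreChanged with the new value.
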(event `self.ReceiveBeginPlay`
  (`KismetSystemLibrary.K2_SetTimer` null "Add Score" 0.5 true))

(event `self.ReceiveTick`
  (params (DeltaSeconds :type "Float (single-precision)")))

(fn `Add Score`
  (bind _returnvalue (`GameplayStatics.GetActorOfClass` "/Game/Blueprints/BP_MyPlayerController.BP_MyPlayerController_C"))
  (if (`/Game/Blueprints/BP_MyPlayerController.Alive` _returnvalue)
    (set `self.MyScore` (+ (`self.MyScore`) 1.0))))

(fn `OnRep_MyScore`
  (`self.onScoreChanged` (`self.MyScore`)))

(fn `UserConstructionScript`)