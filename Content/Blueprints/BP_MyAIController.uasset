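; AI controller that spawns and possesses a BP_MyPawn at its own transform, then steers it relative to the player's pawn.
; Each tick it pushes toward the player when over 100 units away on X or Y, and always runs MovementAI while the player exists.
; MovementAI adds sideways input from the player controller's AxisInput and moves forward, reversing on collision.
; Pawns falling below Z zero are destroyed, and the pawnless controller destroys itself.
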(event `self.ReceiveBeginPlay`
  (bind (_returnvalue_location _returnvalue_rotation _returnvalue_scale) (`KismetMathLibrary.BreakTransform` (`self.GetTransform`)))
  (bind _returnvalue (`|SpawnActorFromClass` "/Game/Blueprints/BP_MyPawn.BP_MyPawn_C" (`KismetMathLibrary.MakeTransform` _returnvalue_location _returnvalue_rotation) "Undefined" "MultiplyWithRoot" self null))
  (if (`KismetSystemLibrary.IsValid` _returnvalue)
    (bind _output_get (set `self.AIPawn` _returnvalue))
    (set `/Game/Blueprints/BP_MyPawn.Scale` _returnvalue_scale _output_get)
    (`self.Possess` _output_get)
    (bind _asbp_my_player_controller (cast `/Game/Blueprints/BP_MyPlayerController` (`GameplayStatics.GetPlayerController` 0)))
    (set `self.PlayerController` _asbp_my_player_controller)))

(event `self.ReceiveTick`
  (params (DeltaSeconds :type "Float (single-precision)"))
  (bind _aipawn (`self.AIPawn`))
  (bind _returnvalue (`self.K2_GetPawn` (`self.PlayerController`)))
  (bind (_returnvalue_x _returnvalue_y _returnvalue_z) (`KismetMathLibrary.BreakVector` (`self.K2_GetActorLocation` (`self.AIPawn`))))
  (bind (_returnvalue_x_2 _returnvalue_y_2) (`KismetMathLibrary.BreakVector` (- (`self.K2_GetActorLocation` (`self.K2_GetPawn` (`self.PlayerController`))) (`self.K2_GetActorLocation` _aipawn))))
  (bind (_returnvalue_x_3 _returnvalue_y_3) (`KismetMathLibrary.BreakVector` (- (`self.K2_GetActorLocation` _returnvalue) (`self.K2_GetActorLocation` (`self.AIPawn`)))))
  (set `self.DSeconds` DeltaSeconds)
  (if (`KismetSystemLibrary.IsValid` (`self.K2_GetPawn`))
    (if (< _returnvalue_z 0.0)
      (`self.K2_DestroyActor` (`self.AIPawn`))
      (else
        (`/Engine/EditorBlueprintResources/StandardMacros.IsValid` _returnvalue
          (:`Is Valid`
            (if (or (> (`KismetMathLibrary.Abs` _returnvalue_x_3) 100.0) (> (`KismetMathLibrary.Abs` _returnvalue_y_3) 100.0))
              (`Pawn.AddMovementInput` _aipawn (`KismetMathLibrary.MakeVector` _returnvalue_x_2 _returnvalue_y_2) (* (`self.DSeconds`) 500.0) false)
              (bind _forward (`self.MovementAI`))
              (if (not _forward)
                (`KismetSystemLibrary.Delay` 0.2))
              (else
                (bind _forward_2 (`self.MovementAI`))
                (if (not _forward_2)
                  (`KismetSystemLibrary.Delay` 0.2))))))))
    (else
      (`self.K2_DestroyActor`))))

(fn `MovementAI`
  (returns (Forward :type Boolean))
  (bind _returnvalue (`self.GetActorForwardVector`))
  (bind _aipawn (`self.AIPawn`))
  (if (`KismetSystemLibrary.IsValid` _aipawn)
    (`Pawn.AddMovementInput` _aipawn (`self.GetActorRightVector` _aipawn) (+ (`MyPlayerController.axis_input` (`self.PlayerController`)) (`self.DSeconds`)) false)
    (if (`/Game/Blueprints/BP_MyPawn.isCollision` (`self.AIPawn`))
      (`Pawn.AddMovementInput` (`self.AIPawn`) _returnvalue (* (`self.DSeconds`) -500.0) false)
      (set `/Game/Blueprints/BP_MyPawn.isCollision` false (`self.AIPawn`))
      (return false)
      (else
        (`Pawn.AddMovementInput` (`self.AIPawn`) _returnvalue (* (`self.DSeconds`) 100.0) false)
        (return true)))))

(fn `UserConstructionScript`)