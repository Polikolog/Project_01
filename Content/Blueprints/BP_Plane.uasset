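; Ground segment actor that fills itself with obstacles and, on player overlap, requests the next plane from PlaneSpawner and destroys itself five seconds later.
; Each time the score reaches a doubling threshold, it spawns a random-shaped BP_Let, plus a BP_Piece if the pawn's scale is low.
; Spawn locations come from random Points children, with a loose occupancy check.
; Spawned obstacles and pieces are tracked and destroyed with the plane.
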(event `self.ReceiveDestroyed`
  (`self.K2_DestroyActor` (`self.Let`))
  (`self.K2_DestroyActor` (`self.Pieces`)))

(event `self.ReceiveBeginPlay`
  (set `self.Plank` 25.0))

(event `self.ReceiveTick`
  (params (DeltaSeconds :type "Float (single-precision)"))
  (bind _returnvalue_x (`KismetMathLibrary.BreakVector` (`self.GetActorScale3D` (`Controller.K2_GetPawn` (`GameplayStatics.GetPlayerController` 0)))))
  (bind _asbp_player_state (cast `/Game/Blueprints/BP_PlayerState` (`GameplayStatics.GetPlayerState` 0)))
  (if (>= (`/Game/Blueprints/BP_PlayerState.MyScore` _asbp_player_state) (`self.Plank`))
    (`self.AddLet`)
    (set `self.Plank` (* (`self.Plank`) 2.0))
    (`self.CreatePiece` _returnvalue_x)))

(event `self.SpawnTrigger.OnComponentBeginOverlap`
  (params (OverlappedComponent :type "PrimitiveComponent Object Reference") (OtherActor :type "Actor Object Reference") (OtherComp :type "PrimitiveComponent Object Reference") (OtherBodyIndex :type Integer) (bFromSweep :type Boolean) (SweepResult :type "HitResult Structure (by ref)"))
  (cast `/Game/Blueprints/BP_MyPawn` OtherActor)
  (`ActorComponent.K2_DestroyComponent` (`self.SpawnTrigger`))
  (`/Game/Blueprints/BP_SpawnPlane.Spawn Plane on Spawn Point` (`self.PlaneSpawner`))
  (`KismetSystemLibrary.Delay` 5.0)
  (`self.K2_DestroyActor`))

(fn `AddLet`
  (locals (NewLocalVar :type "Set of /Game/Blueprints/BP_Let Object Reference"))
  (bind _returnvalue (`self.FindLoc`))
  (bind _returnvalue_2 (`|SpawnActorFromClass` "/Game/Blueprints/BP_Let.BP_Let_C" (`KismetMathLibrary.MakeTransform` _returnvalue (struct :`Yaw` 90.0)) "Undefined" "MultiplyWithRoot" null null))
  (`KismetArrayLibrary.Array_Add` (`self.Let`) _returnvalue_2)
  (`StaticMeshComponent.SetStaticMesh` (`/Game/Blueprints/BP_Let.StaticMesh` _returnvalue_2) (select `int` (`KismetMathLibrary.RandomIntegerInRange` 0 5) :`0` "/Game/Static/Shapes/Shape_Cone.Shape_Cone" :`1` "/Game/Static/Shapes/Shape_Cube.Shape_Cube" :`2` "/Game/Static/Shapes/Shape_Cylinder.Shape_Cylinder" :`3` "/Game/Static/Shapes/Shape_QuadPyramid.Shape_QuadPyramid" :`4` "/Game/Static/Shapes/Shape_Wedge_B.Shape_Wedge_B" :`5` "/Game/Static/Shapes/Shape_WideCapsule.Shape_WideCapsule" :!type "StaticMesh Object Reference")))

(fn `CreatePiece`
  (params (sendScale :type "Float (double-precision)"))
  (if (< sendScale 0.9)
    (bind _returnvalue (`self.FindLoc`))
    (bind _returnvalue_2 (`|SpawnActorFromClass` "/Game/Blueprints/BP_Piece.BP_Piece_C" (`KismetMathLibrary.MakeTransform` (`KismetMathLibrary.MakeVector` (.x _returnvalue) (.y _returnvalue) 10.0)) "Undefined" "MultiplyWithRoot" null null))
    (`KismetArrayLibrary.Array_Add` (`self.Pieces`) _returnvalue_2)
    (set `/Game/Blueprints/BP_Piece.Plane` self _returnvalue_2)))

(fn `FindLoc`
  (returns (ReturnValue :type "Vector Structure"))
  (bind _let (`self.Let`))
  (bind _children (`SceneComponent.GetChildrenComponents` (`self.Points`) false))
  (bind _returnvalue (`SceneComponent.K2_GetComponentLocation` (`|GetArrayItem` _children (`KismetMathLibrary.RandomInteger` (`KismetArrayLibrary.Array_Length` _children)))))
  (if (not (`KismetArrayLibrary.Array_IsEmpty` _let))
    (for _array_element _let
      (if (== (`self.K2_GetActorLocation` _array_element) _returnvalue)
        (break)
        (else
          (return _returnvalue)))))
  (return _returnvalue))

(fn `RandomizeLet`
  (locals (Lets :type "Array of StaticMeshComponent Object Reference"))
  (`self.AddLet`))

(fn `RemoveLet`
  (params (Let :type "/Game/Blueprints/BP_Let Object Reference"))
  (bind _returnvalue (`KismetArrayLibrary.Array_RemoveItem` (`self.Let`) Let))
  (if _returnvalue
    (`self.K2_DestroyActor` Let)))

(fn `UserConstructionScript`)