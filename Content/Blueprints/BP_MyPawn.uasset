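; BP_MyPawn is a physics-sphere pawn that drives itself forward, shrinks on each hit and is destroyed when too small or below zero height.
; Hits reverse movement briefly, pause collision and physics, and spawn a BP_MyAIController actor at a PieceSpawnArea child point, indexed randomly or by overlap checks.
; A RepNotify Scale applies size changes and calls CallOnScaleChange; destroying the pawn also destroys its AI controller.
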(event `self.ReceiveBeginPlay`
  (`self.WhenHit`)
  (set `self.Scale` (`KismetMathLibrary.MakeVector` 1.5 1.5 1.5))
  (`KismetSystemLibrary.Delay` 1.0)
  (`self.AfterHit`)
  (set `self.point num` (`KismetMathLibrary.RandomIntegerInRange` 0 7)))

(event `self.ReceiveTick`
  (params (DeltaSeconds :type "Float (single-precision)"))
  (bind _returnvalue (`self.GetActorForwardVector`))
  (bind (_returnvalue_x _returnvalue_y _returnvalue_z) (`KismetMathLibrary.BreakVector` (`self.K2_GetActorLocation`)))
  (bind _scale_x (`KismetMathLibrary.BreakVector` (`self.Scale`)))
  (if (< _returnvalue_z 0.0)
    (`self.K2_DestroyActor`)
    (elif (< _scale_x 0.2)
      (`self.K2_DestroyActor`)
      (elif (`self.isCollision`)
        (`self.AddMovementInput` _returnvalue (* DeltaSeconds -500.0))
        (`KismetSystemLibrary.Delay` 0.2)
        (set `self.isCollision` false)
        (else
          (`self.AddMovementInput` _returnvalue (* DeltaSeconds (`self.GetForwardSpeed`))))))))

(event `self.Sphere.OnComponentHit`
  (params (HitComponent :type "PrimitiveComponent Object Reference") (OtherActor :type "Actor Object Reference") (OtherComp :type "PrimitiveComponent Object Reference") (NormalImpulse :type "Vector Structure") (Hit :type "HitResult Structure (by ref)"))
  (set `self.isCollision` true)
  (`self.ChangeScale` true)
  (`self.WhenHit`)
  (`self.SpawnAI`)
  (`KismetSystemLibrary.Delay` 2.0)
  (`self.AfterHit`))

(event `self.PieceSpawnArea.OnComponentBeginOverlap`
  (params (OverlappedComponent :type "PrimitiveComponent Object Reference") (OtherActor :type "Actor Object Reference") (OtherComp :type "PrimitiveComponent Object Reference") (OtherBodyIndex :type Integer) (bFromSweep :type Boolean) (SweepResult :type "HitResult Structure (by ref)"))
  (if (not (== OtherActor self))
    (for (_array_element _array_index) (`SceneComponent.GetChildrenComponents` (`self.PieceSpawnArea`) false)
      (bind (_returnvalue_x _returnvalue_y) (`KismetMathLibrary.BreakVector` (- (`SceneComponent.K2_GetComponentLocation` _array_element) (`self.K2_GetActorLocation` OtherActor))))
      (if (not (or (< _returnvalue_x 50.0) (< _returnvalue_y 50.0)))
        (set `self.point num` _array_index)))))

(event `self.ReceiveDestroyed`
  (bind _asbp_my_aicontroller (cast `/Game/Blueprints/BP_MyAIController` (`self.GetController`)))
  (`self.K2_DestroyActor` _asbp_my_aicontroller))

(fn `AfterHit`
  (bind _sphere (`self.Sphere`))
  (`PrimitiveComponent.SetCollisionEnabled` _sphere "QueryAndPhysics")
  (`PrimitiveComponent.SetSimulatePhysics` _sphere true))

(fn `ChangeScale`
  (params (isLoss :type Boolean))
  (bind _scale_x (`KismetMathLibrary.BreakVector` (`self.Scale`)))
  (if isLoss
    ;[1 1 1] decrement scale
    (bind _output_get (set `self.Scale` (- (`self.Scale`) (0.5 0.5 0.5))))
    (`self.AddMovementInput` (`self.GetActorUpVector`) (.z _output_get))
    (elif (< _scale_x 1.5)
      ;[1 1 1] increment scale
      (set `self.Scale` (+ (`self.Scale`) (0.2 0.2 0.2))))))

(fn `OnRep_Scale`
  (bind _scale_x (`KismetMathLibrary.BreakVector` (`self.Scale`)))
  (`self.onScaleChange` _scale_x)
  (`self.SetActorScale3D` (`self.Scale`)))

(fn `SpawnAI`
  (`|SpawnActorFromClass` "/Game/Blueprints/BP_MyAIController.BP_MyAIController_C" (`KismetMathLibrary.MakeTransform` (`SceneComponent.K2_GetComponentLocation` (`|GetArrayItem` (`SceneComponent.GetChildrenComponents` (`self.PieceSpawnArea`) false) (`self.point num`))) (struct) (`self.Scale`)) "Undefined" "MultiplyWithRoot" null null))

(fn `UserConstructionScript`)

(fn `WhenHit`
  (bind _sphere (`self.Sphere`))
  (`PrimitiveComponent.SetSimulatePhysics` _sphere false)
  (`PrimitiveComponent.SetCollisionEnabled` _sphere "NoCollision"))