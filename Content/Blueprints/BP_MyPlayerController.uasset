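; Player controller that manages possession, death and restart in a game built around BP_MyPawn and spawned planes.
; While alive, Tick replaces a lost pawn with the last existing BP_MyPawn, highlighted via custom depth, or clears Alive if none remain.
; Alive's RepNotify broadcasts the state, switching to camera and UI input on death, or game input and Restart, which respawns pawn and plane spawner and resets score.
; Escape quits.
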(event `self.ReceiveBeginPlay`
  (bind _asbp_my_pawn (cast `/Game/Blueprints/BP_MyPawn` (`self.K2_GetPawn`)))
  (`PrimitiveComponent.SetRenderCustomDepth` (`/Game/Blueprints/BP_MyPawn.StaticMesh` _asbp_my_pawn) true))

(event `self.ReceiveTick`
  (params (DeltaSeconds :type "Float (single-precision)"))
  (if (`KismetSystemLibrary.IsValid` (`self.K2_GetPawn`))
    _
    (elif (`self.Alive`)
      (`self.Reborn`))))

(event `Key|Escape`
  (params (Key :type "Key Structure"))
  (:`Pressed`
    (`KismetSystemLibrary.QuitGame` null "Quit")))

(fn `OnRep_Alive`
  (bind _alive (`self.Alive`))
  (`self.AliveEventDispatcher` _alive)
  (if _alive
    (`WidgetBlueprintLibrary.SetInputMode_GameOnly` self)
    (set `self.bShowMouseCursor` false)
    (`self.Restart`)
    (else
      (bind _returnvalue (`GameplayStatics.GetActorOfClass` "/Script/Engine.CameraActor"))
      (`self.SetViewTargetWithBlend` self _returnvalue 0.0 "VTBlend_Linear" 0.0 false)
      (`WidgetBlueprintLibrary.SetInputMode_UIOnlyEx` self null)
      (set `self.bShowMouseCursor` true))))

(fn `Reborn`
  (locals (AliveChanged :type Boolean))
  (bind _outactors (`GameplayStatics.GetAllActorsOfClass` "/Game/Blueprints/BP_MyPawn.BP_MyPawn_C"))
  (if (`KismetArrayLibrary.Array_IsEmpty` _outactors)
    (set `self.Alive` false)
    (else
      (bind _output (`|GetArrayItem` _outactors (`KismetArrayLibrary.Array_LastIndex` _outactors)))
      (set `self.ControlledPawn` _output)
      (`self.Possess` _output)
      (`PrimitiveComponent.SetRenderCustomDepth` (`/Game/Blueprints/BP_MyPawn.StaticMesh` _output) true))))

(fn `Restart`
  (bind _returnvalue (`GameplayStatics.GetActorOfClass` "/Game/Blueprints/BP_SpawnPlane.BP_SpawnPlane_C"))
  (`self.K2_DestroyActor` _returnvalue)
  (bind _outactors (`GameplayStatics.GetAllActorsOfClass` "/Game/Blueprints/BP_Plane.BP_Plane_C"))
  (`self.K2_DestroyActor` _outactors)
  (bind _returnvalue_2 (`GameplayStatics.GetActorOfClass` "/Script/Engine.PlayerStart"))
  (bind _returnvalue_3 (`self.GetTransform` _returnvalue_2))
  (bind _returnvalue_4 (`|SpawnActorFromClass` "/Game/Blueprints/BP_MyPawn.BP_MyPawn_C" _returnvalue_3 "Undefined" "MultiplyWithRoot" null null))
  (`self.Possess` _returnvalue_4)
  (set `/Game/Blueprints/BP_MyPawn.Scale` (1.5 1.5 1.5) _returnvalue_4)
  (`|SpawnActorFromClass` "/Game/Blueprints/BP_SpawnPlane.BP_SpawnPlane_C" _returnvalue_3 "Undefined" "MultiplyWithRoot" null null)
  (bind _asbp_player_state (cast `/Game/Blueprints/BP_PlayerState` (`GameplayStatics.GetPlayerState` 0)))
  (set `/Game/Blueprints/BP_PlayerState.MyScore` 0.0 _asbp_player_state))

(fn `UserConstructionScript`)