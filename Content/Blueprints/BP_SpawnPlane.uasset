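; BP_SpawnPlane is a spawner actor that lays an initial chain of BP_Plane segments when play begins.
; InitSpawn places the first plane at the player pawn's X position, then attaches each following one at the previous plane's SpawnPoint.
; Each new plane is stored as NewPanel, receives a reference back to the spawner and runs RandomizeLet.
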(event `self.ReceiveBeginPlay`
  (`self.InitSpawn`))

(fn `InitSpawn`
  (bind _returnvalue_x (`KismetMathLibrary.BreakVector` (`self.K2_GetActorLocation` (`Controller.K2_GetPawn` (`GameplayStatics.GetPlayerController` 0)))))
  (for _ (range 5)
    (`/Engine/EditorBlueprintResources/StandardMacros.IsValid` (`self.NewPanel`)
      (:`Is Valid`
        (`self.Spawn Plane on Spawn Point`))
      (:`Is Not Valid`
        (`self.Spawn Plane` (`KismetMathLibrary.MakeVector` _returnvalue_x))))))

(fn `Spawn Plane`
  (params (SpawnVector :type "Vector Structure"))
  (bind _returnvalue (`|SpawnActorFromClass` "/Game/Blueprints/BP_Plane.BP_Plane_C" (`KismetMathLibrary.MakeTransform` SpawnVector) "Undefined" "MultiplyWithRoot" null null))
  (bind _output_get (set `self.NewPanel` _returnvalue))
  (set `/Game/Blueprints/BP_Plane.PlaneSpawner` self _output_get)
  (`/Game/Blueprints/BP_Plane.RandomizeLet` _output_get))

(fn `Spawn Plane on Spawn Point`
  (`self.Spawn Plane` (`SceneComponent.K2_GetComponentLocation` (`/Game/Blueprints/BP_Plane.SpawnPoint` (`self.NewPanel`)))))

(fn `UserConstructionScript`)